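; BP_WallChase is a wall actor that pursues the player character along the world Y axis.
; Each tick it takes a normalized direction from the player's location and its own Y, then sweeps its position by CurrentSpeed, keeping X and Z fixed.
; When that direction closely aligns with the player's forward vector, speed rises to BaseSpeed times ChaseSpeedMult and never resets.
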(event EventBeginPlay
  (Variables|Default|SetTargetPlayer (Game|GetPlayerCharacter 0))
  (Variables|Default|SetCurrentSpeed (Variables|Default|GetBaseSpeed)))

(event EventTick
  (params (DeltaSeconds :type Float%20%28single-precision%29))
  (bind _returnvalue (Transformation|GetActorLocation))
  (bind _targetplayer (Variables|Default|GetTargetPlayer))
  (bind _returnvalue_2 (Transformation|GetActorLocation _targetplayer))
  (bind _returnvalue_3 (- _returnvalue_2 (.y _returnvalue)))
  (bind _returnvalue_4 (Math|Vector|Normalize _returnvalue_3 0.1))
  (Transformation|SetActorLocation (Math|Vector|MakeVector (.x _returnvalue) (.y (+ (Transformation|GetActorLocation) (* _returnvalue_4 DeltaSeconds (Variables|Default|GetCurrentSpeed)))) (.z _returnvalue)) true false)
  (bind _output_get (Variables|Default|SetNormalizedWallDirection _returnvalue_4))
  (if (>= (Math|Vector|DotProduct _output_get (Transformation|GetActorForwardVector (Variables|Default|GetTargetPlayer))) 0.7)
    (Variables|Default|SetCurrentSpeed (* (Variables|Default|GetBaseSpeed) (Variables|Default|GetChaseSpeedMult)))))

(fn ConstructionScript)